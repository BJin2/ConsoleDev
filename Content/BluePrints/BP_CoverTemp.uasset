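; BP_CoverTemp is a cover object with Back, Front and Right trigger volumes that tell the player pawn which side it overlaps.
; Begin overlaps call TakeCover, which stores that volume in BP_PlayerPawn's OverlappingCoverVolume.
; End overlaps call LeaveCover, which checks that stored volume matches, then clears a differently named variable, BPOverlappingCoverVolume0.
; Both events print debug Enter/Exit strings.
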(event `self.Back.OnComponentBeginOverlap`
  (params (OverlappedComponent :type "PrimitiveComponent Object Reference") (OtherActor :type "Actor Object Reference") (OtherComp :type "PrimitiveComponent Object Reference") (OtherBodyIndex :type Integer) (bFromSweep :type Boolean) (SweepResult :type "HitResult Structure (by ref)"))
  (`self.TakeCover` OtherActor (`self.Back`)))

(event `self.Back.OnComponentEndOverlap`
  (params (OverlappedComponent :type "PrimitiveComponent Object Reference") (OtherActor :type "Actor Object Reference") (OtherComp :type "PrimitiveComponent Object Reference") (OtherBodyIndex :type Integer))
  (`self.LeaveCover` OtherActor (`self.Back`)))

(event `TakeCover`
  (params (OverlappedActor :type "Actor Object Reference") (OverlappingVolume :type "BoxComponent Object Reference"))
  (bind _asbp_player_pawn (cast `/Game/BluePrints/BP_PlayerPawn` OverlappedActor))
  (set `TPSCharacter.OverlappingCoverVolume` OverlappingVolume _asbp_player_pawn)
  (`KismetSystemLibrary.PrintString` "Enter"))

(event `LeaveCover`
  (params (OverlappedActor :type "Actor Object Reference") (OverlappingVolume :type "BoxComponent Object Reference"))
  (bind _asbp_player_pawn (cast `/Game/BluePrints/BP_PlayerPawn` OverlappedActor))
  (if (== (`TPSCharacter.OverlappingCoverVolume` _asbp_player_pawn) OverlappingVolume)
    (set `/Game/BluePrints/BP_PlayerPawn.BP_OverlappingCoverVolume_0` null _asbp_player_pawn)
    (`KismetSystemLibrary.PrintString` "Exit")))

(event `self.Front.OnComponentBeginOverlap`
  (params (OverlappedComponent :type "PrimitiveComponent Object Reference") (OtherActor :type "Actor Object Reference") (OtherComp :type "PrimitiveComponent Object Reference") (OtherBodyIndex :type Integer) (bFromSweep :type Boolean) (SweepResult :type "HitResult Structure (by ref)"))
  (`self.TakeCover` OtherActor (`self.Front`)))

(event `self.Front.OnComponentEndOverlap`
  (params (OverlappedComponent :type "PrimitiveComponent Object Reference") (OtherActor :type "Actor Object Reference") (OtherComp :type "PrimitiveComponent Object Reference") (OtherBodyIndex :type Integer))
  (`self.LeaveCover` OtherActor (`self.Front`)))

(event `self.Right.OnComponentBeginOverlap`
  (params (OverlappedComponent :type "PrimitiveComponent Object Reference") (OtherActor :type "Actor Object Reference") (OtherComp :type "PrimitiveComponent Object Reference") (OtherBodyIndex :type Integer) (bFromSweep :type Boolean) (SweepResult :type "HitResult Structure (by ref)"))
  (`self.TakeCover` OtherActor (`self.Right`)))

(event `self.Right.OnComponentEndOverlap`
  (params (OverlappedComponent :type "PrimitiveComponent Object Reference") (OtherActor :type "Actor Object Reference") (OtherComp :type "PrimitiveComponent Object Reference") (OtherBodyIndex :type Integer))
  (`self.LeaveCover` OtherActor (`self.Right`)))

(fn `UserConstructionScript`)