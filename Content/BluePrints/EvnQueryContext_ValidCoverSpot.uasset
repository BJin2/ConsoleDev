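; An Environment Query System context that supplies the cover spots currently shielded from the player as an actor set.
; On each call it clears its list, gathers every CoverSpot actor and traces a short line, CoverWidth long, from each toward player pawn 0.
; Spots whose trace hits something on the custom trace channel are kept and returned, with each trace debug-drawn for one frame.
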(fn `ProvideActorsSet`
  (params (QuerierObject :type "Object Object Reference") (QuerierActor :type "Actor Object Reference"))
  (returns (ResultingActorsSet :type "Array of Actor Object Reference"))
  (locals (ValidCoverSpots :type "Array of /Game/BluePrints/CoverSpot Object Reference"))
  (`KismetArrayLibrary.Array_Clear` (`local.ValidCoverSpots`))
  (bind _outactors (`GameplayStatics.GetAllActorsOfClass` "/Game/BluePrints/CoverSpot.CoverSpot_C"))
  (for _array_element _outactors
    (bind _returnvalue (`Actor.K2_GetActorLocation` _array_element))
    (bind (_outhit _returnvalue_2) (`KismetSystemLibrary.LineTraceSingle` :`Start` _returnvalue :`End` (+ _returnvalue (* (`KismetMathLibrary.Normal` (- (`Actor.K2_GetActorLocation` (`GameplayStatics.GetPlayerPawn` 0)) _returnvalue)) (`self.CoverWidth`))) :`TraceChannel` "TraceTypeQuery4" :`DrawDebugType` "ForOneFrame"))
    (if _returnvalue_2
      (`KismetArrayLibrary.Array_Add` (`local.ValidCoverSpots`) _array_element)))
  (return (`local.ValidCoverSpots`)))